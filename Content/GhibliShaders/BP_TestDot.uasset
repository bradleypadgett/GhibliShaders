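; BP_TestDot is a debug test actor that visualizes the dot product between two directions.
; Each tick it draws white debug arrows from its Sphere and Cube components to Sphere1.
; It then prints the dot product of the two unit direction vectors pointing at Sphere1, showing how closely they align.
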(event EventBeginPlay)

(event Collision|EventActorBeginOverlap
  (params (OtherActor :type Actor%20Object%20Reference)))

(event EventTick
  (params (DeltaSeconds :type Float%20%28single-precision%29))
  (Rendering|Debug|DrawDebugArrow (Transformation|GetWorldLocation (Variables|Default|GetSphere)) (Transformation|GetWorldLocation (Variables|Default|GetSphere1)) 0.0 "(R=1.000000,G=1.000000,B=1.000000,A=1.000000)" 0.0 0.0)
  (Rendering|Debug|DrawDebugArrow (Transformation|GetWorldLocation (Variables|Default|GetCube)) (Transformation|GetWorldLocation (Variables|Default|GetSphere1)) 0.0 "(R=1.000000,G=1.000000,B=1.000000,A=1.000000)" 0.0 0.0)
  (Development|PrintString (Utilities|String|ToString(Float) (Math|Vector|DotProduct (Math|Vector|GetUnitDirection(Vector) (Transformation|GetWorldLocation (Variables|Default|GetSphere)) (Transformation|GetWorldLocation (Variables|Default|GetSphere1))) (Math|Vector|GetUnitDirection(Vector) (Transformation|GetWorldLocation (Variables|Default|GetCube)) (Transformation|GetWorldLocation (Variables|Default|GetSphere1))))) true true "(R=1.000000,G=0.000000,B=0.342601,A=1.000000)"))

(fn ConstructionScript)