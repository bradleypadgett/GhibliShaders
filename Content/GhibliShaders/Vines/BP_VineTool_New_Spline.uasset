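; BP_VineTool_New_Spline is a spline-based vine tool Blueprint that supplies target points for vines.
; Generate Vine Target Points gathers the spline's world-space point locations and copies that array into a vector-array struct for each vine.
; Every vine receives identical points, as the point-jitter step is disconnected from execution.
; The construction script only calls its parent, and the event graph holds disabled stubs.
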(event EventBeginPlay
  (|CallParentFunction) ; This node is disabled and will not be called.\nDrag off pins to build functionality.
)

(event Collision|EventActorBeginOverlap
  (params (OtherActor :type Actor%20Object%20Reference))
  (|CallParentFunction OtherActor) ; This node is disabled and will not be called.\nDrag off pins to build functionality.
)

(event EventTick
  (params (DeltaSeconds :type Float%20%28single-precision%29))
  (|CallParentFunction DeltaSeconds) ; This node is disabled and will not be called.\nDrag off pins to build functionality.
)

(fn ConstructionScript
  (|CallParentFunction))

(fn GenerateVineTargetPoints
  (for _index (range 0 (- (Spline|GetNumberOfSplinePoints (Variables|Default|GetSpline)) 1))
    (Utilities|Array|Add (LocalVariables|GetSpline%20Points%20%28Local%29) (Spline|GetLocationatSplinePoint (Variables|Default|GetSpline) _index "World")))
  (for _index_2 (range 0 (- (Variables|Default|GetNumber%20of%20Vines) 1))
    (Utilities|Array|SetArrayElem (LocalVariables|GetVine%20Points%20%28Local%29) _index_2 (Utilities|Struct|MakeSVectorArray (LocalVariables|GetSpline%20Points%20%28Local%29)) true))
  (return (LocalVariables|GetVine%20Points%20%28Local%29)))