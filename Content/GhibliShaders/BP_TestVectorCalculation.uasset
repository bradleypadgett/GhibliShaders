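; Debug actor that visualizes surface-aligned direction math toward a target actor, using arrows and marker spheres.
; Each tick, sphere traces above, then below, snap a sphere to the surface and capture its normal.
; A cross product rotated around that normal gives a tangent toward the target, along which further traces place a second sphere on nearby surface.
; The construction script applies Z offsets and switches material state between previous and current targets.
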(event Custom|hello)

(event EventTick
  (params (DeltaSeconds :type Float%20%28single-precision%29))
  (bind _returnvalue (Transformation|GetActorLocation))
  (bind _returnvalue_2 (Transformation|GetActorLocation))
  (bind _sphere (Variables|Default|GetSphere))
  (bind _sphere_2 (Variables|Default|GetSphere))
  (bind _sphere_3 (Variables|Default|GetSphere))
  (bind _sphere_4 (Variables|Default|GetSphere))
  (bind _saved_target (Variables|Targets|GetSaved%20Target))
  (bind _sphere_5 (Variables|Default|GetSphere))
  (bind _sphere_6 (Variables|Default|GetSphere))
  (bind _sphere_7 (Variables|Default|GetSphere))
  (bind _sphere1 (Variables|Default|GetSphere1))
  (bind _sphere1_2 (Variables|Default|GetSphere1))
  (bind _returnvalue_3 (Transformation|GetWorldLocation _sphere))
  (bind _returnvalue_4 (Transformation|GetWorldLocation _sphere_3))
  (bind _returnvalue_5 (Transformation|GetWorldLocation _sphere_6))
  (bind _returnvalue_6 (Transformation|GetWorldLocation _sphere_2))
  (bind _returnvalue_7 (Transformation|GetWorldLocation _sphere_4))
  (bind _returnvalue_8 (Transformation|GetActorLocation _saved_target))
  (bind _returnvalue_9 (Transformation|GetWorldLocation _sphere_5))
  (bind _returnvalue_10 (Transformation|GetWorldLocation _sphere_7))
  (bind _returnvalue_11 (Transformation|GetWorldLocation _sphere1))
  (bind _returnvalue_12 (Transformation|GetWorldLocation _sphere1_2))
  (Utilities|FlowControl|Sequence
    (:then_0
      (Rendering|Debug|DrawDebugArrow _returnvalue_5 (+ _returnvalue_5 (* (Class|KismetMathLibrary|VectorForward) (Variables|Default|GetArrow%20Length) 0.5)) 2.0 "(R=1.000000,G=0.000000,B=0.000000,A=1.000000)" 0.05 0.25)
      (Rendering|Debug|DrawDebugArrow _returnvalue_3 (+ _returnvalue_3 (* (Class|KismetMathLibrary|VectorRight) (Variables|Default|GetArrow%20Length) 0.5)) 2.0 "(R=0.000000,G=1.000000,B=0.000000,A=1.000000)" 0.05 0.25)
      (Rendering|Debug|DrawDebugArrow _returnvalue_4 (+ _returnvalue_4 (* (Math|Vector|VectorUp) (Variables|Default|GetArrow%20Length) 0.5)) 2.0 "(R=0.000000,G=0.000000,B=1.000000,A=1.000000)" 0.05 0.25)
      (bind _outhit (Collision|SphereTraceByChannel _returnvalue_2 (- _returnvalue_2 "0,0,-50.000000") 2.0 "TraceTypeQuery1" true 0 "None"))
      (if (.bBlockingHit (Collision|BreakHitResult _outhit))
        (Variables|Default|SetImpact%20Point (.ImpactPoint (Collision|BreakHitResult _outhit)))
        (Variables|Default|SetImpact%20Normal (.ImpactNormal (Collision|BreakHitResult _outhit)))
        (Transformation|SetWorldLocation (Variables|Default|GetSphere) (Variables|Default|GetImpact%20Point) false false)
        (Rendering|Material|SetMaterial (Variables|Default|GetSphere) 0 "/Engine/BasicShapes/BasicShapeMaterial.BasicShapeMaterial" :!label _label)
        (Transformation|SetWorldLocation (Variables|Default|GetSphere) (Variables|Default|GetImpact%20Point) false false)
        (Rendering|Debug|DrawDebugArrow _returnvalue_7 (+ _returnvalue_7 (* (Variables|Default|GetImpact%20Normal) (Variables|Default|GetArrow%20Length))) 2.5 "(R=1.000000,G=1.000000,B=0.000000,A=1.000000)" 0.05 0.5) ; Surface Normal
        (else
          (bind _outhit_2 (Collision|SphereTraceByChannel _returnvalue (- _returnvalue "0,0.000000,1000.000000") 2.0 "TraceTypeQuery1" true 0 "ForOneFrame"))
          (if (.bBlockingHit (Collision|BreakHitResult _outhit_2))
            (Variables|Default|SetImpact%20Point (.ImpactPoint (Collision|BreakHitResult _outhit_2)))
            (Variables|Default|SetImpact%20Normal (.ImpactNormal (Collision|BreakHitResult _outhit_2)))
            (goto _label)
            (else
              (Rendering|Material|SetMaterial (Variables|Default|GetSphere) 0 "/Engine/MapTemplates/Materials/BasicAsset01.BasicAsset01")
              (Transformation|SetWorldLocation (Variables|Default|GetSphere) (Transformation|GetActorLocation) false false))))))
    (:then_1
      (if (Utilities|Operators|NotEqual(!=) :A (Variables|Default|GetImpact%20Point) :ErrorTolerance 0.1)
        (Rendering|Debug|DrawDebugArrow _returnvalue_9 _returnvalue_8 1e+01 "(R=0.250000,G=0.250000,B=0.250000,A=1.000000)" 0.05 0.1)
        (Rendering|Debug|DrawDebugArrow _returnvalue_6 (+ _returnvalue_6 (* (Math|Vector|RotateVectorAroundAxis (Math|Vector|Normalize (Math|Vector|CrossProduct (Variables|Default|GetImpact%20Normal) (Math|Vector|GetUnitDirection(Vector) _returnvalue_9 _returnvalue_8))) (- (Variables|Default|GetAngle%20Deg) 9e+01) (Variables|Default|GetImpact%20Normal)) (Variables|Default|GetArrow%20Length) 0.75)) 4.0 "(R=1.000000,G=0.201985,B=0.920566,A=1.000000)" 0.05 0.75)
        (bind _outhit_3 (Collision|SphereTraceByChannel (+ _returnvalue_10 (* (Variables|Default|GetImpact%20Normal) 15)) (+ (* (Math|Vector|Normalize (Math|Vector|GetUnitDirection(Vector) (+ _returnvalue_10 (* (Variables|Default|GetImpact%20Normal) 15)) (+ _returnvalue_10 (* (Math|Vector|RotateVectorAroundAxis (Math|Vector|Normalize (Math|Vector|CrossProduct (Variables|Default|GetImpact%20Normal) (Math|Vector|GetUnitDirection(Vector) (Transformation|GetWorldLocation (Variables|Default|GetSphere)) (Transformation|GetActorLocation (Variables|Targets|GetSaved%20Target))))) -9e+01 (Variables|Default|GetImpact%20Normal)) 15)))) 10) (+ _returnvalue_10 (* (Math|Vector|RotateVectorAroundAxis (Math|Vector|Normalize (Math|Vector|CrossProduct (Variables|Default|GetImpact%20Normal) (Math|Vector|GetUnitDirection(Vector) (Transformation|GetWorldLocation (Variables|Default|GetSphere)) (Transformation|GetActorLocation (Variables|Targets|GetSaved%20Target))))) -9e+01 (Variables|Default|GetImpact%20Normal)) 15))) 2.0 "TraceTypeQuery1" true 0 "None"))
        (if (.bBlockingHit (Collision|BreakHitResult _outhit_3))
          (Rendering|SetVisibility (Variables|Default|GetSphere1) true false)
          (Transformation|SetWorldLocation (Variables|Default|GetSphere1) (.ImpactPoint (Collision|BreakHitResult _outhit_3)) false false)
          (Rendering|Debug|DrawDebugArrow _returnvalue_12 (+ _returnvalue_12 (* (.ImpactNormal (Collision|BreakHitResult _outhit_3)) (Variables|Default|GetArrow%20Length))) 2.5 "(R=1.000000,G=1.000000,B=0.000000,A=1.000000)" 0.05 0.5) ; Surface Normal
          (else
            (bind _outhit_4 (Collision|SphereTraceByChannel (+ (Transformation|GetWorldLocation (Variables|Default|GetSphere)) (* (Math|Vector|RotateVectorAroundAxis (Math|Vector|Normalize (Math|Vector|CrossProduct (Variables|Default|GetImpact%20Normal) (Math|Vector|GetUnitDirection(Vector) (Transformation|GetWorldLocation (Variables|Default|GetSphere)) (Transformation|GetActorLocation (Variables|Targets|GetSaved%20Target))))) (- (Variables|Default|GetAngle%20Deg) 9e+01) (Variables|Default|GetImpact%20Normal)) 15)) (- (+ (Transformation|GetWorldLocation (Variables|Default|GetSphere)) (* (Math|Vector|RotateVectorAroundAxis (Math|Vector|Normalize (Math|Vector|CrossProduct (Variables|Default|GetImpact%20Normal) (Math|Vector|GetUnitDirection(Vector) (Transformation|GetWorldLocation (Variables|Default|GetSphere)) (Transformation|GetActorLocation (Variables|Targets|GetSaved%20Target))))) (- (Variables|Default|GetAngle%20Deg) 9e+01) (Variables|Default|GetImpact%20Normal)) 15)) (Math|Vector|MakeVector 0.0 0.0 (Math|Float|SelectFloat 15.0 -15.0 (> (.z (Variables|Default|GetImpact%20Normal)) 0.0)))) 2.0 "TraceTypeQuery1" true 0 "None"))
            (Rendering|SetVisibility (Variables|Default|GetSphere1) true false)
            (Transformation|SetWorldLocation (Variables|Default|GetSphere1) (.ImpactPoint (Collision|BreakHitResult _outhit_4)) false false)
            (Rendering|Debug|DrawDebugArrow _returnvalue_11 (+ _returnvalue_11 (* (.ImpactNormal (Collision|BreakHitResult _outhit_4)) (Variables|Default|GetArrow%20Length))) 2.5 "(R=1.000000,G=1.000000,B=0.000000,A=1.000000)" 0.05 0.5) ; Surface Normal
          ))))))

(fn ConstructionScript
  (bind _target (Variables|Targets|GetTarget))
  (Transformation|AddRelativeLocation (Variables|Default|GetSphere) (Math|Vector|MakeVector 0.0 0.0 (Variables|Default|GetRelative%20Location%20Z)) false false)
  (Transformation|AddActorWorldOffset (Math|Vector|MakeVector 0.0 0.0 (Variables|Default|GetWorld%20Offset%20Z)))
  (Utilities|IsValid (Variables|Targets|GetSaved%20Target)
    (:Is%20Valid
      (Default|SetMaterial (Variables|Targets|GetSaved%20Target) false))
    (:Is%20Not%20Valid
      _))
  (Utilities|IsValid _target
    (:Is%20Valid
      (Default|SetMaterial _target true)
      (Variables|Targets|SetSaved%20Target (Variables|Targets|GetTarget)))))