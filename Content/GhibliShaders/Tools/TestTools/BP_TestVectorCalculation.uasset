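; Debug test actor for vector math that generates a chain of mesh points along surfaces toward a series of targets.
; A looping timer traces for a start surface, then clears and rebuilds the point chain segment by segment.
; GeneratePoint rotates a cross-product vector around the current normal, sphere-traces the next hit and ends the segment on a miss, backward step or target proximity.
; Debug arrows show world axes, normals, step directions and targets.
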(event Custom|Generation
  (bind _returnvalue (Transformation|GetActorLocation))
  (bind _returnvalue_2 (Transformation|GetActorLocation))
  (bind _sphere (Variables|Default|GetSphere))
  (bind _targets (Variables|Targets|GetTargets))
  (bind _returnvalue_3 (Transformation|GetWorldLocation _sphere))
  (Utilities|FlowControl|Sequence
    (:then_0
      ;[1 1 1] Draw Absolute Coordinate Arrows
      (CallFunction|DrawAbsoluteArrow (Class|KismetMathLibrary|VectorForward) "(R=1.000000,G=0.000000,B=0.000000,A=1.000000)") ; X
      (CallFunction|DrawAbsoluteArrow (Class|KismetMathLibrary|VectorRight) "(R=0.000000,G=1.000000,B=0.000000,A=1.000000)") ; Y
      (CallFunction|DrawAbsoluteArrow (Math|Vector|VectorUp) "(R=0.000000,G=0.000000,B=1.000000,A=1.000000)") ; Y
      (bind _outhit (Collision|SphereTraceByChannel _returnvalue_2 (- _returnvalue_2 "0,0,-50.000000") 2.0 "TraceTypeQuery1" true (Utilities|Array|MakeArray (Variables|/Script/Engine.ChildActorComponent|GetChildActor (Variables|Default|GetChildActor))) "None"))
      (if (.bBlockingHit (Collision|BreakHitResult _outhit))
        (Variables|Default|SetInitial%20Impact%20Point (.ImpactPoint (Collision|BreakHitResult _outhit)))
        (Variables|Default|SetInitial%20Impact%20Normal (.ImpactNormal (Collision|BreakHitResult _outhit)))
        (Transformation|SetWorldLocation (Variables|Default|GetSphere) (Variables|Default|GetInitial%20Impact%20Point) false false)
        (Rendering|Material|SetMaterial (Variables|Default|GetSphere) 0 "/Engine/BasicShapes/BasicShapeMaterial.BasicShapeMaterial" :!label _label)
        (Transformation|SetWorldLocation (Variables|Default|GetSphere) (Variables|Default|GetInitial%20Impact%20Point) false false)
        (Rendering|Debug|DrawDebugArrow _returnvalue_3 (+ _returnvalue_3 (* (Variables|Default|GetInitial%20Impact%20Normal) (Variables|Default|GetArrow%20Length))) 2.5 "(R=1.000000,G=1.000000,B=0.000000,A=1.000000)" 0.1 0.5) ; Surface Normal
        (else
          (bind _outhit_2 (Collision|SphereTraceByChannel _returnvalue (- _returnvalue "0,0.000000,1000.000000") 2.0 "TraceTypeQuery1" true (Utilities|Array|MakeArray (Variables|/Script/Engine.ChildActorComponent|GetChildActor (Variables|Default|GetChildActor))) "ForOneFrame"))
          (if (.bBlockingHit (Collision|BreakHitResult _outhit_2))
            (Variables|Default|SetInitial%20Impact%20Point (.ImpactPoint (Collision|BreakHitResult _outhit_2)))
            (Variables|Default|SetInitial%20Impact%20Normal (.ImpactNormal (Collision|BreakHitResult _outhit_2)))
            (goto _label)
            (else
              (Rendering|Material|SetMaterial (Variables|Default|GetSphere) 0 "/Engine/MapTemplates/Materials/BasicAsset01.BasicAsset01")
              (Transformation|SetWorldLocation (Variables|Default|GetSphere) (Transformation|GetActorLocation) false false))))))
    (:then_1
      (for _array_element (Variables|Default|GetMeshes)
        (Components|DestroyComponent _array_element))
      (Utilities|Array|Clear (Variables|Default|GetMeshes))
      (Utilities|IsValid (Utilities|Array|Get(acopy) _targets)
        (:Is%20Valid
          (if (> (Utilities|Array|Length _targets) 1)
            (if (Utilities|Operators|NotEqual(!=) :A (Variables|Default|GetInitial%20Impact%20Point) :ErrorTolerance 0.1)
              (Variables|Default|SetCurrent%20Point (Variables|Default|GetSphere))
              (Variables|Default|SetCurrent%20Point%20Normal (Variables|Default|GetInitial%20Impact%20Normal))
              (Variables|Default|SetCurrent%20Point%20Location (Variables|Default|GetInitial%20Impact%20Point))
              (for _index (range 1 (- (Utilities|Array|Length (Variables|Targets|GetTargets)) 1))
                (bind _output_get (Variables|Targets|SetCurrent%20Segment _index))
                (Variables|Targets|SetCurrent%20Target%20Direction (Math|Vector|GetUnitDirection(Vector) (Transformation|GetActorLocation (Utilities|Array|Get(acopy) (Variables|Targets|GetTargets) (- (Variables|Targets|GetCurrent%20Segment) 1))) (Transformation|GetActorLocation (Utilities|Array|Get(acopy) (Variables|Targets|GetTargets) (Variables|Targets|GetCurrent%20Segment)))))
                (bind _index_2 (Utilities|FlowControl|ForLoopwithBreak (- (Utilities|Array|Length (Variables|Default|GetMeshes)) 1) (- (Variables|Default|GetGenerated%20Points) 2) :!label _label_2)
                  (:LoopBody
                    (Variables|Default|SetCurrent%20Point%20Index _index_2)
                    (bind _break (CallFunction|GeneratePoint))
                    (if _break
                      (goto _label_2 Break)))
                  (:Completed
                    ;[1 1 1] Arrow to Target
                    (Rendering|Debug|DrawDebugArrow (Transformation|GetWorldLocation (select (<= (Utilities|Array|Length (Variables|Default|GetMeshes)) 1) (Variables|Default|GetSphere) (Utilities|Array|Get(acopy) (Variables|Default|GetMeshes) (- (Utilities|Array|Length (Variables|Default|GetMeshes)) 2)))) (Transformation|GetActorLocation (Utilities|Array|Get(acopy) (Variables|Targets|GetTargets) (Variables|Targets|GetCurrent%20Segment))) 1e+01 "(R=0.991667,G=0.991667,B=0.991667,A=1.000000)" 0.1 0.5) ; Target Arrow
                  ))))))))))

(event EventBeginPlay
  (Utilities|Time|SetTimerbyFunctionName 0 "Generation" 0.1 true))

(fn ConstructionScript
  (Transformation|AddRelativeLocation (Variables|Default|GetSphere) (Math|Vector|MakeVector 0.0 0.0 (Variables|Default|GetRelative%20Location%20Z)) false false)
  (Transformation|AddActorWorldOffset (Math|Vector|MakeVector 0.0 0.0 (Variables|Default|GetWorld%20Offset%20Z)))
  (bind _asbp_test_target (Utilities|Casting|CastToBP_TestTarget (Variables|/Script/Engine.ChildActorComponent|GetChildActor (Variables|Default|GetChildActor))))
  (Utilities|Array|SetArrayElem (Variables|Targets|GetTargets) 0 _asbp_test_target true))

(fn GeneratePoint
  (Rendering|Debug|DrawDebugArrow (Transformation|GetWorldLocation (Variables|Default|GetCurrent%20Point)) (+ (Transformation|GetWorldLocation (Variables|Default|GetCurrent%20Point)) (* (Math|Vector|RotateVectorAroundAxis (Math|Vector|Normalize (Utilities|GetCrossProduct)) -9e+01 (Variables|Default|GetCurrent%20Point%20Normal)) (Variables|Default|GetArrow%20Length) 0.75)) 4.0 "(R=1.000000,G=0.000000,B=0.927830,A=1.000000)" 0.1 0.75)
  (bind _outhit (Collision|SphereTraceByChannel (+ (Transformation|GetWorldLocation (Variables|Default|GetCurrent%20Point)) (* (Variables|Default|GetCurrent%20Point%20Normal) 15)) (+ (* (Math|Vector|Normalize (Math|Vector|GetUnitDirection(Vector) (+ (Transformation|GetWorldLocation (Variables|Default|GetCurrent%20Point)) (* (Variables|Default|GetCurrent%20Point%20Normal) 15)) (+ (Transformation|GetWorldLocation (Variables|Default|GetCurrent%20Point)) (* (Math|Vector|RotateVectorAroundAxis (Utilities|GetCrossProduct) -9e+01 (Variables|Default|GetCurrent%20Point%20Normal)) 15)))) 10) (+ (Transformation|GetWorldLocation (Variables|Default|GetCurrent%20Point)) (* (Math|Vector|RotateVectorAroundAxis (Utilities|GetCrossProduct) -9e+01 (Variables|Default|GetCurrent%20Point%20Normal)) 15))) 2.0 "TraceTypeQuery1" true 0 "ForDuration" true "(R=1.000000,G=0.000000,B=0.000000,A=1.000000)" "(R=0.000000,G=1.000000,B=0.000000,A=1.000000)" 1.0))
  (if (.bBlockingHit (Collision|BreakHitResult _outhit))
    (if (>= (Math|Vector|DotProduct (Math|Vector|GetUnitDirection(Vector) (Variables|Default|GetCurrent%20Point%20Location) (.ImpactPoint (Collision|BreakHitResult _outhit))) (Variables|Targets|GetCurrent%20Target%20Direction)) 0.0)
      (Variables|Default|SetCurrent%20Point%20Location (.ImpactPoint (Collision|BreakHitResult _outhit)))
      (Variables|Default|SetCurrent%20Point%20Normal (.ImpactNormal (Collision|BreakHitResult _outhit)))
      (bind _returnvalue (AddComponent|AddStaticMeshComponent false))
      (bind _output_get (Variables|Default|SetCurrent%20Point _returnvalue))
      (Utilities|Array|Add (Variables|Default|GetMeshes) _output_get)
      (Transformation|SetWorldLocation (Variables|Default|GetCurrent%20Point) (Variables|Default|GetCurrent%20Point%20Location) false false)
      (Rendering|Debug|DrawDebugArrow (Transformation|GetWorldLocation (Variables|Default|GetCurrent%20Point)) (+ (Transformation|GetWorldLocation (Variables|Default|GetCurrent%20Point)) (* (Variables|Default|GetCurrent%20Point%20Normal) (Variables|Default|GetArrow%20Length))) 2.5 "(R=1.000000,G=1.000000,B=0.000000,A=1.000000)" 0.1 0.5) ; Surface Normal
      (return (< (Class|KismetMathLibrary|VectorDistanceSquared (Transformation|GetWorldLocation (Variables|Default|GetCurrent%20Point)) (Transformation|GetActorLocation (Utilities|Array|Get(acopy) (Variables|Targets|GetTargets) (Variables|Targets|GetCurrent%20Segment)))) 2e+01))
      (else
        (return true)))
    (else
      (return true))))

(fn DrawAbsoluteArrow
  (params (In%20Vector :type Vector) (Color :type Linear%20Color%20Structure))
  (bind _sphere (Variables|Default|GetSphere))
  (bind _returnvalue (Transformation|GetWorldLocation _sphere))
  (Rendering|Debug|DrawDebugArrow _returnvalue (+ _returnvalue (* In%20Vector (Variables|Default|GetArrow%20Length) 0.5)) 2.0 Color 0.5 0.25))