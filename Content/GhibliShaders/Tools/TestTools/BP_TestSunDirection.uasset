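; Test tool actor that publishes the level's sun direction to materials through a parameter collection.
; Its construction script finds a DirectionalLight, points an arrow component along the light's forward vector and writes that vector into the "Sun Direction" parameter of MPC_Wind.
; The update only happens when the construction script runs; the event graph does nothing, and leftover debug and math nodes are disconnected.
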(event EventBeginPlay)

(event Collision|EventActorBeginOverlap
  (params (OtherActor :type Actor%20Object%20Reference)))

(event EventTick
  (params (DeltaSeconds :type Float%20%28single-precision%29)))

(fn ConstructionScript
  (bind _returnvalue (Actor|GetActorOfClass "/Script/Engine.DirectionalLight"))
  (Utilities|IsValid _returnvalue
    (:Is%20Valid
      (Development|PrintString "w")
      (Transformation|SetWorldRotation (Variables|Default|GetArrow) (Math|Conversions|RotationFromXVector (Math|Vector|GetForwardVector (Transformation|GetActorRotation _returnvalue))) false false)
      (Rendering|Material|SetVectorParameterValue "/Game/GhibliShaders/Shaders/MPC_Wind.MPC_Wind" "Sun Direction" (Math|Conversions|ToLinearColor(Vector) (Math|Vector|GetForwardVector (Transformation|GetActorRotation _returnvalue))) :!class /Script/Engine.KismetMaterialLibrary))))