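; Debug test actor that visualizes surface normals and tangent directions on the ground beneath its Sphere component.
; Each Tick it line-traces downward, then draws arrows at the hit for the normal, horizontal direction to Target, and slope direction.
; A fourth arrow shows a tangent from the up-cross-normal product, rotated around the normal by AngleDeg.
; Disconnected experiments with sphere traces and dot-product angles remain unexecuted, alongside empty placeholder functions.
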(event Collision|EventActorBeginOverlap
  (params (OtherActor :type Actor%20Object%20Reference)))

(event EventTick
  (params (DeltaSeconds :type Float%20%28single-precision%29))
  (bind _sphere (Variables|Default|GetSphere))
  (bind _target (Variables|Default|GetTarget))
  (bind _returnvalue (Transformation|GetActorLocation _target))
  (bind _returnvalue_2 (Transformation|GetWorldLocation _sphere))
  (bind _outhit (Collision|LineTraceByChannel _returnvalue_2 (- _returnvalue_2 "0,0,100000.000000") "TraceTypeQuery1" true 0 "ForOneFrame" true "(R=0.000000,G=0.338712,B=1.000000,A=1.000000)" "(R=0.000000,G=0.337164,B=1.000000,A=1.000000)"))
  (Variables|Default|SetHit%20Location (.ImpactPoint (Collision|BreakHitResult _outhit)))
  (Variables|Default|SetImpact%20Normal (.Normal (Collision|BreakHitResult _outhit)))
  (Rendering|Debug|DrawDebugArrow (Variables|Default|GetHit%20Location) (+ (Variables|Default|GetHit%20Location) (* (Variables|Default|GetImpact%20Normal) 25)) 4.0 "(R=1.000000,G=1.000000,B=1.000000,A=1.000000)" 0.05 0.5)
  (Rendering|Debug|DrawDebugArrow (Variables|Default|GetHit%20Location) (+ (Variables|Default|GetHit%20Location) (* (Math|Vector|GetUnitDirection(Vector) (Math|Vector|MakeVector (.x (Variables|Default|GetHit%20Location)) (.y (Variables|Default|GetHit%20Location)) 0.0) (Math|Vector|MakeVector (.x _returnvalue) (.y _returnvalue) 0.0)) 25)) 4.0 "(R=0.000000,G=1.000000,B=0.000000,A=1.000000)" 0.05 0.5)
  (Rendering|Debug|DrawDebugArrow (Variables|Default|GetHit%20Location) (+ (Variables|Default|GetHit%20Location) (* (Math|Vector|RotateVectorAroundAxis (Math|Vector|Normalize (Math|Vector|CrossProduct (Math|Vector|VectorUp) (Variables|Default|GetImpact%20Normal))) -9e+01 (Variables|Default|GetImpact%20Normal)) -25)) 4.0 "(R=1.000000,G=0.000000,B=0.000000,A=1.000000)" 0.05 0.5)
  (Rendering|Debug|DrawDebugArrow (Variables|Default|GetHit%20Location) (+ (Variables|Default|GetHit%20Location) (* (Math|Vector|RotateVectorAroundAxis (Math|Vector|Normalize (Math|Vector|CrossProduct (Math|Vector|VectorUp) (Variables|Default|GetImpact%20Normal))) (Variables|Default|GetAngle%20Deg) (Variables|Default|GetImpact%20Normal)) 25)) 4.0 "(R=0.000000,G=0.000000,B=1.000000,A=1.000000)" 0.05 0.5))

(event EventBeginPlay)

(fn ConstructionScript)

(fn NewFunction0)

(fn NewFunction1)

(fn NewFunction2)

(fn NewFunction3)