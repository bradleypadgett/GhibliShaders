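; Editor vine-generation tool that builds vines crawling over surfaces along target paths in its construction script.
; A downward sphere trace finds the starting surface, then forward traces with a wrap-down fallback step along surface tangents, rejecting points heading backward along each segment.
; Each point list initializes a spawned child vine actor.
; Target-point generation, SurfaceTrace and FallingTrace are stubs, and JitterPoints is unused.
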(event EventBeginPlay)

(event Collision|EventActorBeginOverlap
  (params (OtherActor :type Actor%20Object%20Reference)))

(event EventTick
  (params (DeltaSeconds :type Float%20%28single-precision%29)))

(fn ConstructionScript
  (bind _target_points_array (Overrides|GenerateVineTargetPoints))
  (for _array_element _target_points_array
    (Utilities|Array|Clear (Variables|Default|GetGenerated%20Vine%20Points))
    (bind (_generated_vine _vine_points) (Generation|GenerateVineData (Utilities|Struct|BreakSVectorArray _array_element)))
    (if _generated_vine
      (CallFunction|SpawnVine _vine_points))))

(fn GenerateVineTargetPoints
  (return 0))

(fn GenerateVineData
  (params (Target%20Locations :type Array%20of%20Vectors))
  (bind _output_get (LocalVariables|SetTarget%20Locations%20%28Local%29 Target%20Locations))
  (if (>= (Utilities|Array|Length _output_get) 2)
    ;[1 1 1] Get Initial Surface
    (bind (_surface_location _surface_normal _found_surface) (Traces|FindFirstSurface (Utilities|Array|Get(acopy) (LocalVariables|GetTarget%20Locations%20%28Local%29))))
    (if _found_surface
      (Variables|GeneratedPoint|SetCurrent%20Location _surface_location)
      (Variables|GeneratedPoint|SetSurface%20Normal _surface_normal)
      ;[1 1 1] Iterate through each target segment (current index -1 -> current index)
      (for _index (range 1 (- (Utilities|Array|Length (LocalVariables|GetTarget%20Locations%20%28Local%29)) 1))
        (Variables|GeneratedPoint|SetCurrent%20Generation%20Segment _index)
        (Utilities|FlowControl|ForLoopwithBreak 0 50 :!label _label
          (:LoopBody
            (bind (_found_vine_point _generated_location _generated_surface_normal) (Generation|GenerateNextVinePoint (LocalVariables|GetTarget%20Locations%20%28Local%29)))
            (if _found_vine_point
              (Generation|AddNextVinePoint _generated_location _generated_surface_normal)
              (else
                (goto _label Break))))))
      (return true (Variables|Default|GetGenerated%20Vine%20Points))
      (else
        (return false 0)))
    (else
      (return false 0))))

(fn SpawnVine
  (params (Vine%20Points :type Array%20of%20Vectors))
  (LocalVariables|SetVine%20Points%20%28Local%29 Vine%20Points)
  (bind _returnvalue (AddComponent|AddChildActorComponent false))
  (Class|BPIVineTool|InitializeVine(Message) (Variables|/Script/Engine.ChildActorComponent|GetChildActor _returnvalue) (Utilities|Struct|MakeSVineData (LocalVariables|GetVine%20Points%20%28Local%29) 0) (Variables|Default|GetDistance%20Between%20Points)))

(fn SurfaceTrace
  (params (Start%20Location :type Vector) (Surface%20Normal :type Vector) (Target%20Direction :type Vector))
  (return "0, 0, 0" false))

(fn FallingTrace
  (params (Start%20Location :type Vector))
  (return false))

(fn FindFirstSurface
  (params (First%20Target%20Location :type Vector))
  (bind (_return_location _found_surface) (Traces|SurfaceTrace "0, 0, 0" "0, 0, 0" "0, 0, 0"))
  (if _found_surface
    (return _return_location "0, 0, 0" false)
    (else
      (bind _outhit (Collision|SphereTraceByChannel First%20Target%20Location (- First%20Target%20Location "0,0,250.000000") 2.0 "TraceTypeQuery1" true 0 "None"))
      (if (.bBlockingHit (Collision|BreakHitResult _outhit))
        (return (.ImpactPoint (Collision|BreakHitResult _outhit)) (.ImpactNormal (Collision|BreakHitResult _outhit)) true)
        (else
          (return "0, 0, 0" "0, 0, 0" false))))))

(fn GetCurrentSegmentData
  (params (Target%20Locations :type Array%20of%20Vectors))
  (bind _current_generation_segment (Variables|GeneratedPoint|GetCurrent%20Generation%20Segment))
  (bind _current_generation_segment_2 (Variables|GeneratedPoint|GetCurrent%20Generation%20Segment))
  (bind _output (Utilities|Array|Get(acopy) Target%20Locations _current_generation_segment))
  (bind _returnvalue (- _current_generation_segment_2 1))
  (bind _output_2 (Utilities|Array|Get(acopy) Target%20Locations _returnvalue))
  (return (Math|Vector|GetUnitDirection(Vector) _output_2 _output) _output_2 _output))

(fn GenerateNextVinePoint
  (params (Target%20Locations :type Array%20of%20Vectors))
  (bind _current_location (Variables|GeneratedPoint|GetCurrent%20Location))
  (bind _surface_normal (Variables|GeneratedPoint|GetSurface%20Normal))
  (bind _returnvalue (* _surface_normal 15))
  (bind _returnvalue_2 (+ _current_location _returnvalue))
  (LocalVariables|SetTarget%20Locations%20%28Local%29_ Target%20Locations)
  ;[1 1 1] Trace Forward
  (bind _outhit (Collision|SphereTraceByChannel _returnvalue_2 (+ (* (Math|Vector|Normalize (Math|Vector|GetUnitDirection(Vector) _returnvalue_2 (+ (Variables|GeneratedPoint|GetCurrent%20Location) (* (Generation|GetCurrentPointTangent (LocalVariables|GetTarget%20Locations%20%28Local%29_)) 15)))) 10) (+ (Variables|GeneratedPoint|GetCurrent%20Location) (* (Generation|GetCurrentPointTangent (LocalVariables|GetTarget%20Locations%20%28Local%29_)) 15))) 2.0 "TraceTypeQuery1" true 0 "None" true "(R=1.000000,G=0.000000,B=0.000000,A=1.000000)" "(R=0.000000,G=1.000000,B=0.000000,A=1.000000)" 1.0))
  (if (.bBlockingHit (Collision|BreakHitResult _outhit))
    (if (Generation|ValidateVinePoint (.ImpactPoint (Collision|BreakHitResult _outhit)) (.ImpactNormal (Collision|BreakHitResult _outhit)) (LocalVariables|GetTarget%20Locations%20%28Local%29_))
      (return true (.ImpactPoint (Collision|BreakHitResult _outhit)) (.ImpactNormal (Collision|BreakHitResult _outhit)))
      (else
        _)))
  (bind _outhit_2 (Collision|SphereTraceByChannel (+ (Variables|GeneratedPoint|GetCurrent%20Location) (* (Variables|GeneratedPoint|GetSurface%20Normal) 10) (* (Generation|GetCurrentPointTangent (LocalVariables|GetTarget%20Locations%20%28Local%29_)) 5)) (+ (Variables|GeneratedPoint|GetCurrent%20Location) (* (Variables|GeneratedPoint|GetSurface%20Normal) -10)) 2.0 "TraceTypeQuery1" true 0 "ForDuration" true "(R=1.000000,G=0.000000,B=0.000000,A=1.000000)" "(R=0.000000,G=1.000000,B=0.000000,A=1.000000)" 1.0))
  (if (.bBlockingHit (Collision|BreakHitResult _outhit_2))
    (if (Generation|ValidateVinePoint (.ImpactPoint (Collision|BreakHitResult _outhit_2)) (.ImpactNormal (Collision|BreakHitResult _outhit_2)) (LocalVariables|GetTarget%20Locations%20%28Local%29_))
      (return true (.ImpactPoint (Collision|BreakHitResult _outhit_2)) (.ImpactNormal (Collision|BreakHitResult _outhit_2))))))

(fn ValidateVinePoint
  (params (Location :type Vector) (Surface%20Normal :type Vector) (Target%20Locations :type Array%20of%20Vectors))
  (if (>= (Math|Vector|DotProduct (Math|Vector|GetUnitDirection(Vector) (Variables|GeneratedPoint|GetCurrent%20Location) Location) (.Target%20Direction (Generation|GetCurrentSegmentData Target%20Locations))) -0.05)
    (return true)
    (else
      (return false))))

(fn AddNextVinePoint
  (params (Location :type Vector) (Surface%20Normal :type Vector))
  (Variables|GeneratedPoint|SetCurrent%20Location Location)
  (Variables|GeneratedPoint|SetSurface%20Normal Surface%20Normal)
  (Utilities|Array|Add (Variables|Default|GetGenerated%20Vine%20Points) (Variables|GeneratedPoint|GetCurrent%20Location)))

(fn GetCurrentPointTangent
  (params (Target%20Locations :type Array%20of%20Vectors))
  (return (Math|Vector|RotateVectorAroundAxis (Math|Vector|Normalize (Math|Vector|CrossProduct (Variables|GeneratedPoint|GetSurface%20Normal) (Math|Vector|GetUnitDirection(Vector) (Variables|GeneratedPoint|GetCurrent%20Location) (.First%20Target%20Location (Generation|GetCurrentSegmentData Target%20Locations))))) -9e+01 (Variables|GeneratedPoint|GetSurface%20Normal))))

(fn JitterPoints
  (params (Points :type Array%20of%20Vectors) (Jitter%20Amount :type Float%20%28double-precision%29))
  (bind _returnvalue (Math|Float|Absolute(Float) Jitter%20Amount))
  (bind _returnvalue_2 (* _returnvalue -1.0))
  (for _array_element Points
    (Utilities|Array|Add (LocalVariables|GetNew%20Points%20%28Local%29) (+ _array_element (Math|Vector|MakeVector (Math|Random|RandomFloatinRange _returnvalue_2 _returnvalue) (Math|Random|RandomFloatinRange _returnvalue_2 _returnvalue) (Math|Random|RandomFloatinRange _returnvalue_2 _returnvalue)))))
  (return (LocalVariables|GetNew%20Points%20%28Local%29)))