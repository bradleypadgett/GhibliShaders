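; Vine actor that turns supplied vine point data into a mesh that follows a spline.
; InitializeVine rebuilds the master spline from those points, using a minimum-distance check to thin out closely spaced ones.
; It then destroys the existing spline mesh components and creates one per spline segment, matching each segment's positions and tangents.
; The construction script and Tick do nothing, so the vine builds only when InitializeVine is called.
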(event EventTick
  (params (DeltaSeconds :type Float%20%28single-precision%29)))

(event EventInitializeVine
  (params (Vine%20Data :type S%20Vine%20Data%20Structure) (Distance%20Between%20Points :type Float%20%28double-precision%29))
  (Variables|Default|SetDistance%20Between%20Points Distance%20Between%20Points)
  (Utilities|FlowControl|Sequence
    (:then_0
      (Variables|Default|SetVine%20Points (.Points (Utilities|Struct|BreakSVineData Vine%20Data)))
      (Spline|ClearSplinePoints (Variables|Default|GetMaster%20Spline) true)
      (for (_array_element _array_index) (Variables|Default|GetVine%20Points)
        (if (> (- _array_index 1) -1)
          (if (> (Math|Vector|Distance(Vector) (Utilities|Array|Get(acopy) (Variables|Default|GetVine%20Points) (- _array_index 1)) (Variables|Default|GetCurrent%20Point)) (Variables|Default|GetDistance%20Between%20Points))
            (bind _output_get (Variables|Default|SetCurrent%20Point _array_element :!label _label))
            (Spline|AddSplinePoint (Variables|Default|GetMaster%20Spline) _output_get "World" true))
          (else
            (goto _label)))))
    (:then_1
      (CallFunction|ResetVineMesh))))

(fn ConstructionScript)

(fn InitializeVineMesh
  (bind _master_spline (Variables|Default|GetMaster%20Spline))
  (bind _master_spline_2 (Variables|Default|GetMaster%20Spline))
  (Components|StaticMesh|SetStaticMesh (Variables|Default|GetInstancedStaticMesh) (Variables|Default|GetMesh))
  (for _index (range 0 (- (Spline|GetNumberOfSplinePoints (Variables|Default|GetMaster%20Spline)) 2))
    (bind _returnvalue (AddComponent|AddSplineMeshComponent false))
    (bind _output_get (LocalVariables|SetCurrent%20Spline%20Mesh%20Component _returnvalue))
    (Utilities|Array|Add (Variables|Default|GetSpline%20Mesh%20Components) _output_get)
    (Components|StaticMesh|SetStaticMesh (LocalVariables|GetCurrent%20Spline%20Mesh%20Component) (Variables|Default|GetMesh))
    (SplineMesh|SetForwardAxis (LocalVariables|GetCurrent%20Spline%20Mesh%20Component) "X" true)
    (SplineMesh|SetStartandEnd (LocalVariables|GetCurrent%20Spline%20Mesh%20Component) (Spline|GetLocationatSplinePoint _master_spline _index "Local") (Spline|GetTangentatSplinePoint _master_spline _index "Local") (Spline|GetLocationatSplinePoint _master_spline_2 (+ _index 1) "Local") (Spline|GetTangentatSplinePoint _master_spline_2 (+ _index 1) "Local") false :!class /Script/Engine.SplineMeshComponent)))

(fn ResetVineMesh
  (for _array_element (Variables|Default|GetSpline%20Mesh%20Components)
    (Components|DestroyComponent _array_element))
  (CallFunction|InitializeVineMesh))