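; Vine tool Blueprint that generates vine data from a spline, as the spline-driven variant of a vine tool.
; Generate Vines Data loops once per requested vine, gets the points of Spline1, jitters them by a fixed amount and builds a single vine from them.
; It returns the collected vines, while the construction script only calls its parent and the event graph is unused.
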(event EventBeginPlay
  (|CallParentFunction) ; This node is disabled and will not be called.\nDrag off pins to build functionality.
)

(event Collision|EventActorBeginOverlap
  (params (OtherActor :type Actor%20Object%20Reference))
  (|CallParentFunction OtherActor) ; This node is disabled and will not be called.\nDrag off pins to build functionality.
)

(event EventTick
  (params (DeltaSeconds :type Float%20%28single-precision%29))
  (|CallParentFunction DeltaSeconds) ; This node is disabled and will not be called.\nDrag off pins to build functionality.
)

(fn ConstructionScript
  (|CallParentFunction))

(fn GenerateVinesData
  (for _index (range 0 (- (Variables|Default|GetNumber%20of%20Vines) 1))
    (bind _points (CallFunction|GetSplinePoints (Variables|Default|GetSpline1)))
    (CallFunction|JitterPoints _points 25.0)
    (bind _vine_data (CallFunction|GenerateSingleVine _points))
    (Utilities|Array|Add (LocalVariables|GetVines%20Data%20%28Local%29) _vine_data))
  (return (LocalVariables|GetVines%20Data%20%28Local%29)))