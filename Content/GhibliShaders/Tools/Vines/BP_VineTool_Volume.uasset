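; Vine tool variant that scatters randomly shaped vines inside a box volume.
; The construction script sizes the box from Bounds before running the parent's construction.
; GenerateVinesData draws four random points in the box per vine, stores each as actor location minus point, and passes them to GenerateSingleVine to build the returned vine list.
; BeginPlay only adds a debug print of the box extent.
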(event EventBeginPlay
  (|CallParentFunction)
  (Development|PrintString (Utilities|String|ToString(Vector) (.BoxExtent (Collision|GetComponentBounds (Variables|Default|GetBox))))))

(event Collision|EventActorBeginOverlap
  (params (OtherActor :type Actor%20Object%20Reference))
  (|CallParentFunction OtherActor) ; This node is disabled and will not be called.\nDrag off pins to build functionality.
)

(event EventTick
  (params (DeltaSeconds :type Float%20%28single-precision%29))
  (|CallParentFunction DeltaSeconds) ; This node is disabled and will not be called.\nDrag off pins to build functionality.
)

(fn ConstructionScript
  (Components|Box|SetBoxExtent (Variables|Default|GetBox) (Variables|Default|GetBounds) true)
  (|CallParentFunction))

(fn GenerateVinesData
  (for _index (range 0 (- (Variables|Default|GetNumber%20of%20Vines) 1))
    (Utilities|Array|Clear (LocalVariables|GetPoint%20Data%20%28Local%29))
    (for _index_2 (range 0 3)
      (Utilities|Array|Add (LocalVariables|GetPoint%20Data%20%28Local%29) (- (Transformation|GetActorLocation) (Math|Random|RandomPointinBoundingBox (.Origin (Collision|GetComponentBounds (Variables|Default|GetBox))) (Variables|Default|GetBounds)))))
    (bind _vine_data (CallFunction|GenerateSingleVine (LocalVariables|GetPoint%20Data%20%28Local%29)))
    (Utilities|Array|Add (LocalVariables|GetNewLocalVar_0) _vine_data))
  (return (LocalVariables|GetNewLocalVar_0)))