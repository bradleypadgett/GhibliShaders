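; Landscape projection tool actor that shows a texture map on a plane and projects it downward as a decal.
; The construction script creates dynamic materials for both, feeding them the texture plus background and grid mask thresholds and colors.
; It sizes both from the texture's pixel dimensions and a size scale, with a distance scale for decal depth and optional corner-anchored offset.
; BeginPlay only prints the texture size.
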(event EventBeginPlay
  (bind _texture_map (Variables|Mask|GetTexture%20Map))
  (Development|PrintString (Utilities|String|Append "Size X: " (Utilities|String|ToString(Integer) (Class|Texture2D|BlueprintGetSizeX _texture_map)) "Size Y: " (Utilities|String|ToString(Integer) (Class|Texture2D|BlueprintGetSizeY _texture_map)))))

(event Collision|EventActorBeginOverlap
  (params (OtherActor :type Actor%20Object%20Reference)))

(event EventTick
  (params (DeltaSeconds :type Float%20%28single-precision%29)))

(fn ConstructionScript
  (bind _texture_map (Variables|Mask|GetTexture%20Map))
  (bind _projection_size_scale (Variables|Projection|GetProjection%20Size%20Scale))
  (bind _projection_size_scale_2 (Variables|Projection|GetProjection%20Size%20Scale))
  (bind _project_on_corner (Variables|Projection|GetProject%20on%20Corner))
  (bind _texture_map_2 (Variables|Mask|GetTexture%20Map))
  (bind _returnvalue (Class|Texture2D|BlueprintGetSizeX _texture_map_2))
  (bind _returnvalue_2 (Class|Texture2D|BlueprintGetSizeY _texture_map_2))
  (bind _returnvalue_3 (Class|Texture2D|BlueprintGetSizeX _texture_map))
  (bind _returnvalue_4 (Class|Texture2D|BlueprintGetSizeY _texture_map))
  (bind _returnvalue_5 (Math|Conversions|ToFloat(Integer) _returnvalue_3))
  (bind _returnvalue_6 (Math|Conversions|ToFloat(Integer) _returnvalue_4))
  (bind _returnvalue_7 (Math|Conversions|ToFloat(Integer) _returnvalue))
  (bind _returnvalue_8 (Math|Conversions|ToFloat(Integer) _returnvalue_2))
  (bind _returnvalue_9 (Math|Vector|MakeVector _returnvalue_5 _returnvalue_6 0.0))
  (bind _returnvalue_10 (* _projection_size_scale_2 (Math|Vector|MakeVector _returnvalue_7 _returnvalue_8 1.0) 0.01))
  (bind (_x _y) (Math|Vector|BreakVector _returnvalue_10))
  (bind _returnvalue_11 (* _returnvalue_9 0.5 _projection_size_scale))
  (bind _returnvalue_12 (Math|Vector|SelectVector _returnvalue_11 "0, 0, 0" _project_on_corner))
  (bind _returnvalue_13 (Rendering|Material|CreateDynamicMaterialInstance "/Game/GhibliShaders/Landscape/M_Projection_Translucent.M_Projection_Translucent" "None" "None" :!class /Script/Engine.KismetMaterialLibrary))
  (Variables|Default|SetDecal%20Material _returnvalue_13)
  (bind _returnvalue_14 (Rendering|Material|CreateDynamicMaterialInstance "/Game/GhibliShaders/Landscape/M_Projection.M_Projection" "None" "None" :!class /Script/Engine.KismetMaterialLibrary))
  (Variables|Default|SetPlane%20Material _returnvalue_14)
  (Rendering|Components|Decal|SetDecalMaterial (Variables|Default|GetDecal) (Variables|Default|GetDecal%20Material))
  (Rendering|Material|SetMaterial (Variables|Default|GetPlane) 0 (Variables|Default|GetPlane%20Material))
  (Rendering|Material|SetScalarParameterValue (Variables|Default|GetDecal%20Material) "Background Mask Threshold" (Variables|Mask|Background|GetBackground%20Mask%20Threshold) :!class /Script/Engine.MaterialInstanceDynamic)
  (Rendering|Material|SetScalarParameterValue (Variables|Default|GetDecal%20Material) "Grid Mask Threshold" (Variables|Mask|Grid|GetGrid%20Mask%20Threshold) :!class /Script/Engine.MaterialInstanceDynamic)
  (Rendering|Material|SetVectorParameterValue (Variables|Default|GetDecal%20Material) "Background Color" (Variables|Mask|Background|GetBackground%20Color) :!class /Script/Engine.MaterialInstanceDynamic)
  (Rendering|Material|SetVectorParameterValue (Variables|Default|GetDecal%20Material) "Grid Color" (Variables|Mask|Grid|GetGrid%20Color) :!class /Script/Engine.MaterialInstanceDynamic)
  (Rendering|Material|SetTextureParameterValue (Variables|Default|GetDecal%20Material) "Texture" (Variables|Mask|GetTexture%20Map))
  (Transformation|SetWorldScale3D (Variables|Default|GetPlane) _returnvalue_10)
  (Transformation|SetWorldScale3D (Variables|Default|GetDecal) (Math|Vector|RotateVector (Math|Vector|MakeVector _x _y (* (Variables|Projection|GetProjection%20Distance%20Scale) 5.0)) (Variables|/Script/Engine.SceneComponent|GetRelativeRotation (Variables|Default|GetDecal))))
  (Transformation|SetRelativeLocation (Variables|Default|GetDecal) (Math|Vector|MakeVector (.x _returnvalue_12) (.y _returnvalue_12) (* -5e+02 (Variables|Projection|GetProjection%20Distance%20Scale))) false false)
  (Transformation|SetRelativeLocation (Variables|Default|GetPlane) (Math|Vector|MakeVector (.x _returnvalue_12) (.y _returnvalue_12) 0.0) false false))