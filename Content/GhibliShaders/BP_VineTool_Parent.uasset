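; Vine tool parent Blueprint that procedurally builds ivy vines in the construction script, spawning a child actor per vine and passing it points and a mesh.
; The path generator steps between target points with sphere traces, falling until it hits geometry, then probing along the surface, and stores actor-relative points.
; It is unfinished: only one origin point is passed in, skipping tracing, and spline and jitter helpers are not called.
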(event EventBeginPlay)

(event Collision|EventActorBeginOverlap
  (params (OtherActor :type Actor%20Object%20Reference)))

(event EventTick
  (params (DeltaSeconds :type Float%20%28single-precision%29)))

(fn ConstructionScript
  (CallFunction|GenerateVineSeed (Variables|Seed|GetSeed))
  (bind _vine_data (VineData|Override|GenerateVinesData))
  (CallFunction|SpawnVines _vine_data))

(fn GetLastSplinePoint
  (bind _spline (Variables|Default|GetSpline))
  (return (Spline|GetLocationatSplinePoint _spline (Spline|GetNumberOfSplinePoints _spline) "World")))

(fn SetCurrentPointData
  (params (Hit :type Hit%20Result%20Structure))
  (Variables|Spline|Private|SetCurrent%20Position (.location Hit))
  (Variables|Default|SetCurrent%20Point%20Surface%20Normal (.normal Hit))
  (return))

(fn GenerateVinesData
  (bind _vine_data (VineData|GenerateSingleVine (Utilities|Array|MakeArray "0, 0, 0")))
  (return (Utilities|Array|MakeArray _vine_data)))

(fn InitializeVine
  (params (Vine%20Data :type Array%20of%20S%20Vine%20Data%20Structures))
  (return))

(fn GenerateVineSeed
  (params (Seed :type Integer))
  (Math|Random|SetRandomStreamSeed (Variables|Seed|GetMy%20Stream) Seed))

(fn SpawnVines
  (params (Vine%20Data :type Array%20of%20S%20Vine%20Data%20Structures))
  (for _array_element Vine%20Data
    (LocalVariables|SetCurrent%20Vine%20Data%20%28Local%29 _array_element)
    (bind _returnvalue (AddComponent|AddChildActorComponent false))
    (Class|BPIVineTool|InitializeVine(Message) (Variables|/Script/Engine.ChildActorComponent|GetChildActor _returnvalue) (LocalVariables|GetCurrent%20Vine%20Data%20%28Local%29))))

(fn GenerateSingleVine
  (params (Target%20Points%20 :type Array%20of%20Vectors))
  (Variables|Default|SetTarget%20Points Target%20Points%20)
  (if (> (Utilities|Array|Length (Variables|Default|GetTarget%20Points)) 1) ; Check if there's at least 2 points to work with
    (Utilities|Array|Add (LocalVariables|GetGenerated%20Points) (Utilities|Struct|MakeSPoint (Utilities|Array|Get(acopy) (Variables|Default|GetTarget%20Points)) "0.000000,0.000000,0.000000" "0.000000,0.000000,0.000000"))
    (for _index (range 0 (- (Utilities|Array|Length (Variables|Default|GetTarget%20Points)) 2)) ; Each loop will generate points between the\ncurrent target point and next target point
      (bind _output_get (Variables|Default|SetCurrent%20Point (select (== _index 0) (Utilities|Struct|MakeSPoint (Utilities|Array|Get(acopy) (Variables|Default|GetTarget%20Points) _index) "0.000000,0.000000,1.000000" "0.000000,0.000000,0.000000") (Variables|Default|GetCurrent%20Point)))) ; Only swaps out current point at 0 index
      (Variables|Default|SetTarget%20Point (Utilities|Array|Get(acopy) (Variables|Default|GetTarget%20Points) (+ _index 1)))
      (bind _output_get_2 (Variables|Default|SetTarget%20Unit%20Direction (Math|Vector|GetUnitDirection(Vector) (Math|Vector|SelectVector (Utilities|Array|Get(acopy) (Variables|Default|GetTarget%20Points) _index) (.location (Variables|Default|GetCurrent%20Point)) (== _index 0)) (Utilities|Array|Get(acopy) (Variables|Default|GetTarget%20Points) (+ _index 1)))))
      (bind _generated_segment_points (CallFunction|GenerateSegmentPoints))
      (Utilities|Array|AppendArray (LocalVariables|GetGenerated%20Points) _generated_segment_points))
    (Development|PrintString "GENERATED POINTS: " true true "(R=1.000000,G=0.000000,B=0.843845,A=1.000000)" 1e+01)
    (for _array_element (LocalVariables|GetGenerated%20Points)
      (bind _returnvalue (Utilities|Array|Add (LocalVariables|GetGenerated%20Points%20%28Local%29) (- (.Location (Utilities|Struct|BreakSPoint _array_element)) (Transformation|GetActorLocation))))
      (Development|PrintString (Utilities|String|Append (Utilities|String|ToString(Integer) _returnvalue) ": " (Utilities|String|ToString(Vector) (.Location (Utilities|Struct|BreakSPoint _array_element)))) true true "(R=1.000000,G=0.000000,B=0.843845,A=1.000000)" 1e+01))
    (return (Utilities|Struct|MakeSVineData (LocalVariables|GetGenerated%20Points%20%28Local%29) "/Game/Megascans/3D_Plants/English_Ivy_rkEit/S_English_Ivy_rkEit_Var5_lod1.S_English_Ivy_rkEit_Var5_lod1"))
    (else
      (return (Utilities|Struct|MakeSVineData (Variables|Default|GetTarget%20Points) "/Game/Megascans/3D_Plants/English_Ivy_rkEit/S_English_Ivy_rkEit_Var5_lod1.S_English_Ivy_rkEit_Var5_lod1")))))

(fn GetSplinePoints
  (params (Spline :type Spline%20Component%20Object%20Reference))
  (for _index (range 0 (- (Spline|GetNumberOfSplinePoints Spline) 1))
    (Utilities|Array|Add (LocalVariables|GetPoints%20%28Local%29) (Spline|GetLocationatSplinePoint Spline _index "World")))
  (return (LocalVariables|GetPoints%20%28Local%29)))

(fn JitterPoints
  (params (Points :type Array%20of%20Vectors) (Jitter%20Amount :type Float%20%28double-precision%29))
  (bind _returnvalue (Math|Float|Absolute(Float) Jitter%20Amount))
  (bind _returnvalue_2 (* _returnvalue -1.0))
  (for _array_element Points
    (Utilities|Array|Add (LocalVariables|GetNew%20Points%20%28Local%29) (+ _array_element (Math|Vector|MakeVector (Math|Random|RandomFloatinRange _returnvalue_2 _returnvalue) (Math|Random|RandomFloatinRange _returnvalue_2 _returnvalue) (Math|Random|RandomFloatinRange _returnvalue_2 _returnvalue)))))
  (return (LocalVariables|GetNew%20Points%20%28Local%29)))

(fn FallingTrace
  (bind _current_point (Variables|Default|GetCurrent%20Point))
  (bind _current_point_2 (Variables|Default|GetCurrent%20Point))
  (bind _target_unit_direction (Variables|Default|GetTarget%20Unit%20Direction))
  (bind _returnvalue (* _target_unit_direction 25))
  (bind (_x _y _z) (Math|Vector|BreakVector _returnvalue))
  (bind _hit (Utilities|AttemptTrace (.location _current_point_2) (+ (.location _current_point_2) (Math|Vector|MakeVector _x _y (- _z 25.0))) 2.0 "None")
    (:Success
      (return false _hit))
    (:Fail
      (bind _hit_2 (Utilities|AttemptTrace (.location _current_point) (+ (.location _current_point) "0,0,-25.000000") 2.0 "None")
        (:Success
          (return false _hit_2))
        (:Fail
          (return true _hit_2))))))

(fn SurfaceTrace
  (bind _current_point (Variables|Default|GetCurrent%20Point))
  (bind _target_point (Variables|Default|GetTarget%20Point))
  (bind _returnvalue (- (.location _current_point) _target_point))
  (bind _hit (Utilities|AttemptTrace (.location _current_point) (+ (.location _current_point) (* (Math|Vector|Normalize (Math|Vector|CrossProduct (Variables|Default|GetTarget%20Unit%20Direction) (Math|Vector|MakeVector (.x _returnvalue) (.y _returnvalue) 0.0))) 25)) 2.0 "ForDuration")
    (:Success
      _)
    (:Fail
      _))
  (return false _hit))

(fn GetCurrentSegment
  (params (Target%20Points :type Array%20of%20Vectors) (Current%20Index :type Integer) (Generated%20Points :type Array%20of%20S%20Point%20Structures))
  (return (select (== Current%20Index 0) (Utilities|Array|Get(acopy) Generated%20Points (- (Utilities|Array|Length Generated%20Points) 1)) (Utilities|Struct|MakeSPoint (Utilities|Array|Get(acopy) Target%20Points) "0.000000,0.000000,0.000000" "0.000000,0.000000,0.000000")) "0, 0, 0" (Math|Vector|GetUnitDirection(Vector) (Utilities|Array|Get(acopy) (Variables|Default|GetTarget%20Points) Current%20Index) (Utilities|Array|Get(acopy) (Variables|Default|GetTarget%20Points) (+ Current%20Index 1)))))

(fn CheckifPointIsonSurface
  (params (Point%20Location :type S%20Point%20Structure))
  (bind _location (Utilities|Struct|BreakSPoint Point%20Location))
  (Utilities|AttemptTrace _location _location 4.0 "None"
    (:Success
      (return true))
    (:Fail
      (return false))))

(fn GenerateSegmentPoints
  (Variables|Default|SetbFalling true)
  (for _index (range 0 10)
    (bind _near_target_point (CallFunction|CheckNearTargetPoint (Variables|Default|GetCurrent%20Point) (Variables|Default|GetTarget%20Point) 5e+01))
    (bind _output_get (LocalVariables|SetNear%20Target%20Point%20%28Local%29 _near_target_point))
    (if (not _output_get)
      (if (Variables|Default|GetbFalling)
        (bind (_continue_falling _generated_hit) (CallFunction|FallingTrace))
        (bind _output_get_2 (Variables|Default|SetbFalling _continue_falling))
        (if _output_get_2
          (Utilities|Array|AddUnique (LocalVariables|GetGenerated%20Segment%20Points%20%28Local%29) (Utilities|Struct|MakeSPoint (.TraceEnd (Collision|BreakHitResult _generated_hit)) "0.000000,0.000000,1.000000" "0.000000,0.000000,0.000000"))
          (Variables|Default|SetCurrent%20Point (Utilities|Struct|MakeSPoint (.TraceEnd (Collision|BreakHitResult _generated_hit)) "0.000000,0.000000,1.000000" "0.000000,0.000000,0.000000"))
          (else
            (Utilities|Array|AddUnique (LocalVariables|GetGenerated%20Segment%20Points%20%28Local%29) (Utilities|Struct|MakeSPoint (.ImpactPoint (Collision|BreakHitResult _generated_hit)) (.ImpactNormal (Collision|BreakHitResult _generated_hit)) "0.000000,0.000000,0.000000"))
            (Variables|Default|SetCurrent%20Point (Utilities|Struct|MakeSPoint (.ImpactPoint (Collision|BreakHitResult _generated_hit)) (.ImpactNormal (Collision|BreakHitResult _generated_hit)) "0.000000,0.000000,0.000000"))))
        (else
          (bind (_can_t_find_surface_point _generated_hit_2) (CallFunction|SurfaceTrace))
          (bind _output_get_3 (Variables|Default|SetbFalling _can_t_find_surface_point))
          (if _output_get_3
            (bind _on_surface (CallFunction|CheckifPointIsonSurface (Variables|Default|GetCurrent%20Point)))
            (Variables|Default|SetCan't%20Reach%20Target _on_surface)
            (else
              (Utilities|Array|Add (LocalVariables|GetGenerated%20Segment%20Points%20%28Local%29) (Utilities|Struct|MakeSPoint (.ImpactPoint (Collision|BreakHitResult _generated_hit_2)) (.ImpactNormal (Collision|BreakHitResult _generated_hit_2)) "0.000000,0.000000,0.000000"))
              (Variables|Default|SetCurrent%20Point (Utilities|Struct|MakeSPoint (.ImpactPoint (Collision|BreakHitResult _generated_hit_2)) (.ImpactNormal (Collision|BreakHitResult _generated_hit_2)) "0.000000,0.000000,0.000000"))))))))
  (return (LocalVariables|GetGenerated%20Segment%20Points%20%28Local%29)))

(fn CheckNearTargetPoint
  (params (Current%20Point :type S%20Point%20Structure) (Target%20Point :type Vector) (Distance%20Threshold :type Float%20%28double-precision%29))
  (return (<= (Math|Vector|Distance(Vector) (.Location (Utilities|Struct|BreakSPoint Current%20Point)) Target%20Point) (Math|Float|Absolute(Float) Distance%20Threshold))))