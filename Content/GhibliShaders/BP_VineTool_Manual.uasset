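; Manual variant of a vine tool actor in GhibliShaders that supplies hand-authored vine paths.
; Generate Vine Data returns a hard-coded array of two SVineData entries, each a short list of 3D points.
; The construction script only calls its parent, and the event graph holds only disabled default events, so this file does no vine building itself.
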(event EventBeginPlay
  (|CallParentFunction) ; This node is disabled and will not be called.\nDrag off pins to build functionality.
)

(event Collision|EventActorBeginOverlap
  (params (OtherActor :type Actor%20Object%20Reference))
  (|CallParentFunction OtherActor) ; This node is disabled and will not be called.\nDrag off pins to build functionality.
)

(event EventTick
  (params (DeltaSeconds :type Float%20%28single-precision%29))
  (|CallParentFunction DeltaSeconds) ; This node is disabled and will not be called.\nDrag off pins to build functionality.
)

(fn ConstructionScript
  (|CallParentFunction))

(fn GenerateVineData
  (return (Utilities|Array|MakeArray (Utilities|Struct|MakeSVineData (Utilities|Array|MakeArray "0, 0, 0" "10.000000,20.000000, 0" "20.000000,40.000000, 0" "25.000000,50.000000,10.000000") 0) (Utilities|Struct|MakeSVineData (Utilities|Array|MakeArray "-50.000000, 0,5.000000" "20.000000,10.000000,0.000000" "50.000000,20.000000,-5.000000") 0))))