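; Vine actor that lays a chain of mesh segments along a spline, which its owner can supply with the mesh through spawn data.
; The construction script divides spline length by mesh Z size, then adds Z-forward spline mesh components with matched positions and tangents.
; The instanced mesh receives the mesh but no instances.
; Play-time logic is debug only: a printed segment ratio and a drawn sphere trace at Time along the spline.
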(event EventBeginPlay
  (bind _mesh (Variables|Default|GetMesh))
  (bind _returnvalue (StaticMesh|GetBoundingBox _mesh))
  (Development|PrintString (Utilities|String|ToString(Float) (/ (Spline|GetSplineLength (Variables|Default|GetMaster%20Spline)) (.z (- (.max _returnvalue) (.min _returnvalue))))) true true "(R=1.000000,G=0.000000,B=0.120886,A=1.000000)"))

(event Collision|EventActorBeginOverlap
  (params (OtherActor :type Actor%20Object%20Reference)))

(event EventTick
  (params (DeltaSeconds :type Float%20%28single-precision%29))
  (bind _master_spline (Variables|Default|GetMaster%20Spline))
  (bind _time (Variables|Default|GetTime))
  (bind _master_spline_2 (Variables|Default|GetMaster%20Spline))
  (bind _returnvalue (Spline|GetSplineLength _master_spline))
  (bind _returnvalue_2 (* _returnvalue _time))
  (bind _returnvalue_3 (Spline|GetLocationatDistanceAlongSpline _master_spline_2 _returnvalue_2 "World"))
  (Collision|SphereTraceByChannel _returnvalue_3 (+ _returnvalue_3 "0,0,50.000000") 5.0 "TraceTypeQuery1" true 0 "ForOneFrame"))

(fn ConstructionScript
  (bind _mesh (Variables|Default|GetMesh))
  (bind _master_spline (Variables|Default|GetMaster%20Spline))
  (bind _returnvalue (StaticMesh|GetBoundingBox _mesh))
  (bind _returnvalue_2 (Spline|GetSplineLength _master_spline))
  (bind _returnvalue_3 (- (.max _returnvalue) (.min _returnvalue)))
  (bind _returnvalue_4 (/ _returnvalue_2 (.z _returnvalue_3)))
  (bind _returnvalue_5 (Math|Float|Round _returnvalue_4))
  (bind _vine_data (Class|BPIVineTool|CheckforSpawnData(Message) (Components|GetOwner)))
  (CallFunction|SetSpawnData _vine_data)
  (Components|StaticMesh|SetStaticMesh (Variables|Default|GetInstancedStaticMesh) (Variables|Default|GetMesh))
  (for _index (range 0 _returnvalue_5)
    (bind _returnvalue_6 (AddComponent|AddSplineMeshComponent false))
    (Components|StaticMesh|SetStaticMesh _returnvalue_6 (Variables|Default|GetMesh))
    (SplineMesh|SetForwardAxis _returnvalue_6 "Z" true)
    (SplineMesh|SetStartandEnd _returnvalue_6 (Spline|GetLocationatDistanceAlongSpline (Variables|Default|GetMaster%20Spline) (* (Spline|GetSplineLength (Variables|Default|GetMaster%20Spline)) (Math|Float|Clamp(Float) (/ (Math|Conversions|ToFloat(Integer) _index) (Math|Conversions|ToFloat(Integer) _returnvalue_5)))) "Local") (Spline|GetTangentatDistanceAlongSpline (Variables|Default|GetMaster%20Spline) (* (Spline|GetSplineLength (Variables|Default|GetMaster%20Spline)) (Math|Float|Clamp(Float) (/ (Math|Conversions|ToFloat(Integer) _index) (Math|Conversions|ToFloat(Integer) _returnvalue_5)))) "Local") (Spline|GetLocationatDistanceAlongSpline (Variables|Default|GetMaster%20Spline) (* (Spline|GetSplineLength (Variables|Default|GetMaster%20Spline)) (Math|Float|Clamp(Float) (/ (Math|Conversions|ToFloat(Integer) (+ _index 1)) (Math|Conversions|ToFloat(Integer) _returnvalue_5)))) "Local") (Spline|GetTangentatDistanceAlongSpline (Variables|Default|GetMaster%20Spline) (* (Spline|GetSplineLength (Variables|Default|GetMaster%20Spline)) (Math|Float|Clamp(Float) (/ (Math|Conversions|ToFloat(Integer) (+ _index 1)) (Math|Conversions|ToFloat(Integer) _returnvalue_5)))) "Local") true :!class /Script/Engine.SplineMeshComponent)))

(fn SetSpawnData
  (params (Spawn%20Data :type S%20Vine%20Spawn%20Data%20Structure))
  (bind (_spline _mesh) (Utilities|Struct|BreakSVineSpawnData Spawn%20Data))
  (Utilities|IsValid (.Spline (Utilities|Struct|BreakSVineSpawnData Spawn%20Data))
    (:Is%20Valid
      (Variables|Default|SetMaster%20Spline _spline)
      (Variables|Default|SetMesh _mesh)
      (return true))
    (:Is%20Not%20Valid
      (return false))))